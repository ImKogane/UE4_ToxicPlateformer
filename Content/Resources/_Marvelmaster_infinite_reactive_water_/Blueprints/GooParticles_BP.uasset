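; GooParticles_BP is a Blueprint that lets the mouse wheel adjust the jet distance of a goo particle effect.
; Wheel up raises JetDistance and wheel down lowers it by a fixed step, and BeginPlay also runs the lowering step once.
; Each change writes the particle system's "aaa" vector parameter, with X as the distance and Z as negative half of it.
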(event `self.ReceiveBeginPlay`
  (bind _returnvalue (- (`self.JetDistance`) 100.0))
  (`ParticleSystemComponent.SetVectorParameter` (`self.ParticleSystem`) "aaa" (`KismetMathLibrary.MakeVector` _returnvalue 0.0 (* _returnvalue -0.5)) :!label _label)
  (set `self.JetDistance` _returnvalue))

(event `Key|MouseScrollDown` :consume false :overrideparent false
  (params (Key :type "Key Structure"))
  (:`Pressed`
    (goto _label)))

(event `Key|MouseScrollUp`
  (params (Key :type "Key Structure"))
  (bind _returnvalue (+ (`self.JetDistance`) 100.0))
  (:`Pressed`
    (`ParticleSystemComponent.SetVectorParameter` (`self.ParticleSystem`) "aaa" (`KismetMathLibrary.MakeVector` _returnvalue 0.0 (* _returnvalue -0.5)))
    (set `self.JetDistance` _returnvalue)))

(fn `UserConstructionScript`)