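; BP_EndBench is the end-of-game bench that shows key progress and sends the player to the end screen level.
; It binds to the HazardPlayer's get-key event, turning the next of four key components yellow each time.
; On overlap, if the player passes the HasAbilities(7) check and holds at least one key, it adds a fade widget and opens the level after a short delay.
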(event `self.ReceiveBeginPlay`
  (bind _returnvalue (`GameplayStatics.GetActorOfClass` "/Game/ThirdPersonBP/Blueprints/HazardPlayer.HazardPlayer_C"))
  (bind _output_get (set `self.Player` _returnvalue))
  (add `/Game/ThirdPersonBP/Blueprints/HazardPlayer.OnGetKey` _output_get (delegate `NewKey`)))

(event `NewKey`
  (`|ExecutionSequence`
    (:`then_0`
      (`PrimitiveComponent.SetMaterial` (select `int` (`self.Progress`) :`0` (`self.Key`) :`1` (`self.Key1`) :`2` (`self.Key2`) :`3` (`self.Key3`)) 0 "/Game/Materials/M_Yellow.M_Yellow"))
    (:`then_1`
      (`/Engine/EditorBlueprintResources/StandardMacros.IncrementInt` (`self.Progress`)))))

(event `self.Collision.OnComponentBeginOverlap`
  (params (OverlappedComponent :type "PrimitiveComponent Object Reference") (OtherActor :type "Actor Object Reference") (OtherComp :type "PrimitiveComponent Object Reference") (OtherBodyIndex :type Integer) (bFromSweep :type Boolean) (SweepResult :type "HitResult Structure (by ref)"))
  (bind _ashazard_player (cast `/Game/ThirdPersonBP/Blueprints/HazardPlayer` OtherActor))
  (if (and (`HazardCharacter.HasAbilities` _ashazard_player 7) (>= (`/Game/ThirdPersonBP/Blueprints/HazardPlayer.KeyCount` _ashazard_player) 1))
    (bind _returnvalue (`|CreateWidget` "/Game/HUD/HUD_Fade.HUD_Fade_C" (`GameplayStatics.GetPlayerController` 0)))
    (`UserWidget.AddToViewport` _returnvalue 0)
    (`KismetSystemLibrary.Delay` 0.5)
    (`GameplayStatics.OpenLevelBySoftObjectPtr` "/Game/PolygonCity/Maps/EndScreenLevel.EndScreenLevel")))

(fn `UserConstructionScript`)