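; BP_ToxicPile2 is a toxic pile hazard that damages overlapping actors and can be washed away with water for points.
; Actor overlaps start and stop damage through damagePlayer, passing DamageAmount.
; While a "Water"-tagged component overlaps DamageZone, Tick lerps the pile's scale toward zero.
; Once small enough, it awards score, spawns an explosion effect and destroys itself.
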(event `self.ReceiveActorBeginOverlap`
  (params (OtherActor :type "Actor Object Reference"))
  (`/Game/ThirdPersonBP/Blueprints/BPML.DamagePlayer` OtherActor (stale `self.ReceiveActorEndOverlap` OtherActor) (`self.DamageAmount`) :!label _label))

(event `self.ReceiveActorEndOverlap`
  (params (OtherActor :type "Actor Object Reference"))
  (goto _label :!via `ExecEnd`))

(event `self.DamageZone.OnComponentBeginOverlap`
  (params (OverlappedComponent :type "PrimitiveComponent Object Reference") (OtherActor :type "Actor Object Reference") (OtherComp :type "PrimitiveComponent Object Reference") (OtherBodyIndex :type Integer) (bFromSweep :type Boolean) (SweepResult :type "HitResult Structure (by ref)"))
  (if (`ActorComponent.ComponentHasTag` OtherComp "Water")
    (set `self.IsDamaged` true)))

(event `self.DamageZone.OnComponentEndOverlap`
  (params (OverlappedComponent :type "PrimitiveComponent Object Reference") (OtherActor :type "Actor Object Reference") (OtherComp :type "PrimitiveComponent Object Reference") (OtherBodyIndex :type Integer))
  (if (`ActorComponent.ComponentHasTag` OtherComp "Water")
    (set `self.IsDamaged` false)))

(event `self.ReceiveTick`
  (params (DeltaSeconds :type "Float (single-precision)"))
  (bind _returnvalue (`self.GetActorScale3D`))
  (if (`self.IsDamaged`)
    (`self.SetActorScale3D` (`KismetMathLibrary.VLerp` _returnvalue (0.0 0.0 0.0) (* DeltaSeconds 1.5)))
    (if (<= (`KismetMathLibrary.VSize` _returnvalue) 0.8)
      (`/Game/ThirdPersonBP/Blueprints/BPFL.AddScore` 5)
      (`GameplayStatics.SpawnEmitterAtLocation` "/Game/PolygonCity/FX/FX_Explosion.FX_Explosion" (`self.K2_GetActorLocation`))
      (`self.K2_DestroyActor`))))

(fn `UserConstructionScript`)