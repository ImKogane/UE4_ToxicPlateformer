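; BP_CleanSoda is a pickup that temporarily lets the player pass through every BP_Fence in the level.
; When a ThirdPersonCharacter overlaps its Box, it disables collision on all fences, hides itself and switches off its trigger.
; After a DuréeEffet delay, it restores fence collision and reappears with its trigger active again, ready for reuse.
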(event `self.ReceiveActorBeginOverlap`
  (params (OtherActor :type "Actor Object Reference")))

(event `self.Box.OnComponentBeginOverlap`
  (params (OverlappedComponent :type "PrimitiveComponent Object Reference") (OtherActor :type "Actor Object Reference") (OtherComp :type "PrimitiveComponent Object Reference") (OtherBodyIndex :type Integer) (bFromSweep :type Boolean) (SweepResult :type "HitResult Structure (by ref)"))
  (bind _elements (`self.Elements`))
  (cast `/Game/ThirdPersonBP/Blueprints/ThirdPersonCharacter` OtherActor)
  (bind _outactors (`GameplayStatics.GetAllActorsOfClass` "/Game/Blueprints/BP_Fence.BP_Fence_C"))
  (set `self.Elements` _outactors)
  (`self.SetActorEnableCollision` _elements false)
  (`self.SetActorHiddenInGame` true)
  (`PrimitiveComponent.SetCollisionEnabled` (`self.Box`) "NoCollision")
  (`KismetSystemLibrary.Delay` (`self.DuréeEffet`))
  (`self.SetActorEnableCollision` _elements true)
  (`self.SetActorHiddenInGame` false)
  (`PrimitiveComponent.SetCollisionEnabled` (`self.Box`) "QueryOnly"))

(fn `UserConstructionScript`)