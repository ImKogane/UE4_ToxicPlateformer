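; BP_RandomPlayerSkin picks a random player skin and shows it on the main menu model.
; On BeginPlay it draws a mesh and a material independently from ModelsList and MaterialsList, then applies them to MainMenuModel's skeletal mesh component, with the material in the first slot.
; It then saves both picks to BP_MainGameInstance as PlayerModel and PlayerMaterial, so the choice persists across level loads.
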(event `self.ReceiveBeginPlay`
  (bind _skeletalmeshcomponent (`SkeletalMeshActor.SkeletalMeshComponent` (`self.MainMenuModel`)))
  (set `self.ChoosedModel` (`KismetArrayLibrary.Array_Random` (`self.ModelsList`)))
  (set `self.ChoosedMaterial` (`KismetArrayLibrary.Array_Random` (`self.MaterialsList`)))
  (`SkinnedMeshComponent.SetSkinnedAssetAndUpdate` _skeletalmeshcomponent (`self.ChoosedModel`) true)
  (`PrimitiveComponent.SetMaterial` _skeletalmeshcomponent 0 (`self.ChoosedMaterial`))
  (bind _asbp_main_game_instance (cast `/Game/Blueprints/BP_MainGameInstance` (`GameplayStatics.GetGameInstance`)))
  (set `/Game/Blueprints/BP_MainGameInstance.PlayerModel` (`self.ChoosedModel`) _asbp_main_game_instance)
  (set `/Game/Blueprints/BP_MainGameInstance.PlayerMaterial` (`self.ChoosedMaterial`) _asbp_main_game_instance))

(fn `UserConstructionScript`)