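; Wooden-sounding platform that reacts when a HazardPlayer steps on its top trigger by either bouncing or falling, chosen by the Falls flag.
; Bounce drives the mesh and its separate collider vertically with a timeline, guarded by a DoOnce until it finishes.
; Fall plays a timed yaw animation, switches the mesh to physics simulation, then after a delay restores collision and snaps it back to the root.
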(event `self.TopCollision.OnComponentBeginOverlap`
  (params (OverlappedComponent :type "PrimitiveComponent Object Reference") (OtherActor :type "Actor Object Reference") (OtherComp :type "PrimitiveComponent Object Reference") (OtherBodyIndex :type Integer) (bFromSweep :type Boolean) (SweepResult :type "HitResult Structure (by ref)"))
  (cast `/Game/ThirdPersonBP/Blueprints/HazardPlayer` OtherActor)
  (`GameplayStatics.PlaySoundAtLocation` "/Game/Sounds/wood_crack.wood_crack" (`self.K2_GetActorLocation`) (struct) 0.3 1.0 0.0 null null null)
  (if (`self.Falls`)
    (`self.Fall`)
    (else
      (`self.Bounce`))))

(event `Bounce`
  (`/Engine/EditorBlueprintResources/StandardMacros.DoOnce` false :!label _label
    (:`Completed`
      (`TimelineComponent.SetPlayRate` (`self.Timeline_0`) (/ 1.0 (`self.BounceSpeed`)))
      (bind (_direction _newtrack_1) (`Timeline|Timeline_0` :!via `PlayFromStart`)
        (:`Update`
          (bind _returnvalue (* (* (0.0 0.0 1.0) (`self.MoveStrength`)) _newtrack_1))
          (`SceneComponent.K2_SetRelativeLocation` (`self.PlatformCollision`) (+ _returnvalue (0.0 0.0 10.0)) false false)
          (`SceneComponent.K2_SetRelativeLocation` (`self.Platform`) _returnvalue false false))
        (:`Finished`
          (goto _label :!via `Reset`))))))

(event `Fall`
  (bind (_returnvalue_location _returnvalue_rotation) (`KismetMathLibrary.BreakTransform` (`SceneComponent.K2_GetComponentToWorld` (`self.Root`))))
  (`PrimitiveComponent.SetCollisionEnabled` (`self.TopCollision`) "NoCollision")
  (`TimelineComponent.SetPlayRate` (`self.Timeline_1`) (/ 1.0 (`self.FallDelay`)))
  (bind (_direction _newtrack_1) (`Timeline|Timeline_1` :!via `PlayFromStart`)
    (:`Update`
      (`SceneComponent.K2_SetRelativeRotation` (`self.Platform`) (* (* (`KismetMathLibrary.MakeRotator` 0.0 0.0 1.0) (`self.MoveStrength`)) _newtrack_1) false false))
    (:`Finished`
      (`PrimitiveComponent.SetCollisionProfileName` (`self.Platform`) "BlockAllDynamic" true)
      (`PrimitiveComponent.SetSimulatePhysics` (`self.Platform`) true)
      (`PrimitiveComponent.SetCollisionEnabled` (`self.PlatformCollision`) "NoCollision")
      (`KismetSystemLibrary.Delay` (`self.FallResetDelay`))
      (`PrimitiveComponent.SetCollisionEnabled` (`self.TopCollision`) "QueryAndPhysics")
      (`PrimitiveComponent.SetCollisionEnabled` (`self.PlatformCollision`) "QueryAndPhysics")
      (`PrimitiveComponent.SetSimulatePhysics` (`self.Platform`) false)
      (`PrimitiveComponent.SetCollisionProfileName` (`self.Platform`) "NoCollision" true)
      (`KismetSystemLibrary.Delay` 0.2)
      (`SceneComponent.K2_SetWorldLocationAndRotation` (`self.Platform`) _returnvalue_location _returnvalue_rotation false false))))

(fn `UserConstructionScript`)