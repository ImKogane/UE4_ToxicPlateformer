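; Water container that fills while a Water-tagged component overlaps its capsule, moving a linked actor toward a destination actor's starting location.
; Tick steps a clamped Progress value that drives both the Water mesh's Z scale and the linked actor's position lerp, without delta-time scaling.
; A timer re-armed during filling delays draining, which then reverses both effects down to empty.
; Its widget rotates every tick to face the HazardPlayer's follow camera.
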(event `self.ReceiveBeginPlay`
  (bind _water (`self.Water`))
  (bind (_relativescale3d_x _relativescale3d_y _relativescale3d_z) (`KismetMathLibrary.BreakVector` (`SceneComponent.RelativeScale3D` _water)))
  (`|ExecutionSequence`
    (:`then_0`
      (bind _objecttomove (`self.ObjectToMove`)
        (:`then`
          (set `self.OriginalPosition` (`self.K2_GetActorLocation` _objecttomove)))
        (:`else`)))
    (:`then_1`
      (bind _objectdestination (`self.ObjectDestination`)
        (:`then`
          (set `self.OriginalDestination` (`self.K2_GetActorLocation` _objectdestination)))
        (:`else`)))
    (:`then_2`
      (set `self.TargetScale` _relativescale3d_z)
      (`SceneComponent.SetRelativeScale3D` _water (`KismetMathLibrary.MakeVector` _relativescale3d_x _relativescale3d_y)))
    (:`then_3`
      (bind _returnvalue (`GameplayStatics.GetActorOfClass` "/Game/ThirdPersonBP/Blueprints/HazardPlayer.HazardPlayer_C"))
      (set `self.Player` _returnvalue))))

(event `self.Capsule.OnComponentBeginOverlap`
  (params (OverlappedComponent :type "PrimitiveComponent Object Reference") (OtherActor :type "Actor Object Reference") (OtherComp :type "PrimitiveComponent Object Reference") (OtherBodyIndex :type Integer) (bFromSweep :type Boolean) (SweepResult :type "HitResult Structure (by ref)"))
  (if (`ActorComponent.ComponentHasTag` OtherComp "Water")
    (set `self.IsColliding` true)))

(event `self.Capsule.OnComponentEndOverlap`
  (params (OverlappedComponent :type "PrimitiveComponent Object Reference") (OtherActor :type "Actor Object Reference") (OtherComp :type "PrimitiveComponent Object Reference") (OtherBodyIndex :type Integer))
  (if (`ActorComponent.ComponentHasTag` OtherComp "Water")
    (set `self.IsColliding` false)))

(event `self.ReceiveTick`
  (params (DeltaSeconds :type "Float (single-precision)"))
  (bind _widget (`self.Widget`))
  (`|ExecutionSequence`
    (:`then_0`
      (if (`self.IsColliding`)
        (`self.Fill`)
        (`KismetSystemLibrary.K2_SetTimerDelegate` (delegate `StartToEmpty`) (`self.TimeoutDelay`))
        (set `self.CanEmpty` false :!label _label)
        (elif (`self.CanEmpty`)
          (`self.Empty`)
          (if (<= (`self.Progress`) 0.0)
            (goto _label)))))
    (:`then_1`
      (`SceneComponent.K2_SetWorldRotation` _widget (`KismetMathLibrary.FindLookAtRotation` (`SceneComponent.K2_GetComponentLocation` _widget) (`SceneComponent.K2_GetComponentLocation` (`/Game/ThirdPersonBP/Blueprints/HazardPlayer.FollowCamera` (`self.Player`)))) false false))))

(event `StartToEmpty`
  (set `self.CanEmpty` true))

(event `Fill`
  (bind _water (`self.Water`))
  (bind (_relativescale3d_x _relativescale3d_y) (`KismetMathLibrary.BreakVector` (`SceneComponent.RelativeScale3D` _water)))
  (set `self.Progress` (`KismetMathLibrary.FClamp` (+ (`self.Progress`) (`self.ProgressSpeed`))))
  (`|ExecutionSequence` :!label _label_2
    (:`then_0`
      (bind _objecttomove (`self.ObjectToMove`)
        (:`then`
          (`self.K2_SetActorLocation` _objecttomove (`KismetMathLibrary.VLerp` (`self.OriginalPosition`) (`self.OriginalDestination`) (`self.Progress`)) false false))
        (:`else`)))
    (:`then_1`
      (`SceneComponent.SetRelativeScale3D` _water (`KismetMathLibrary.MakeVector` _relativescale3d_x _relativescale3d_y (`KismetMathLibrary.Lerp` 0.0 (`self.TargetScale`) (`self.Progress`))))
      (`SceneComponent.SetHiddenInGame` (`self.Water`) (<= (`self.Progress`) 0.0) false))))

(event `Empty`
  (set `self.Progress` (`KismetMathLibrary.FClamp` (- (`self.Progress`) (`self.ProgressSpeed`))))
  (goto _label_2))

(fn `UserConstructionScript`)