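; BP_Laser is a hazard actor: a laser that switches on and off and damages what touches it.
; After an initial TimeToStart delay, BeginPlay loops indefinitely, using the same Timer delay for the off and on phases.
; Each phase change toggles LaserMesh visibility together with Box collision between query-only and disabled.
; Any actor that begins overlapping the Box takes damage once per overlap, with no filtering by actor type.
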(event `self.ReceiveBeginPlay`
  (`KismetSystemLibrary.Delay` (`self.TimeToStart`))
  (`KismetSystemLibrary.Delay` (`self.timer`) :!label _label)
  (`SceneComponent.SetVisibility` (`self.LaserMesh`) true false)
  (`PrimitiveComponent.SetCollisionEnabled` (`self.Box`) "QueryOnly")
  (`KismetSystemLibrary.Delay` (`self.timer`))
  (`SceneComponent.SetVisibility` (`self.LaserMesh`) false false)
  (`PrimitiveComponent.SetCollisionEnabled` (`self.Box`) "NoCollision")
  (goto _label))

(event `self.Box.OnComponentBeginOverlap`
  (params (OverlappedComponent :type "PrimitiveComponent Object Reference") (OtherActor :type "Actor Object Reference") (OtherComp :type "PrimitiveComponent Object Reference") (OtherBodyIndex :type Integer) (bFromSweep :type Boolean) (SweepResult :type "HitResult Structure (by ref)"))
  (`GameplayStatics.ApplyDamage` OtherActor 1.0 null self))

(fn `UserConstructionScript`)