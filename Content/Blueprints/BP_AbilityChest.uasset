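; BP_AbilityChest is a locked chest that grants a HazardPlayer abilities in exchange for a key.
; On overlap it calls RemoveKey, and on success unlocks the AbilitiesToUnlock bitmask, disables its collision and swaps the closed mesh for the opened one.
; The first matching bit (Toxic, Jetpack, then Soda) selects one reward mesh, which a timeline moves along Z before destroying it.
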(event `self.Collision.OnComponentBeginOverlap`
  (params (OverlappedComponent :type "PrimitiveComponent Object Reference") (OtherActor :type "Actor Object Reference") (OtherComp :type "PrimitiveComponent Object Reference") (OtherBodyIndex :type Integer) (bFromSweep :type Boolean) (SweepResult :type "HitResult Structure (by ref)"))
  (bind _ashazard_player (cast `/Game/ThirdPersonBP/Blueprints/HazardPlayer` OtherActor))
  (bind _removedkey (`/Game/ThirdPersonBP/Blueprints/HazardPlayer.RemoveKey` _ashazard_player))
  (if _removedkey
    (`HazardCharacter.UnlockAbilities` _ashazard_player (`self.AbilitiesToUnlock`))
    (`PrimitiveComponent.SetCollisionEnabled` (`self.Collision`) "NoCollision")
    (`SceneComponent.SetHiddenInGame` (`self.ChestClosed`) true false)
    (`SceneComponent.SetHiddenInGame` (`self.ChestOpened`) false false)
    (if (`KismetMathLibrary.Conv_IntToBool` (`KismetMathLibrary.And_IntInt` (`self.AbilitiesToUnlock`) (`|BitmaskLiteral` 1)))
      ;[1 1 1] Toxic
      (`SceneComponent.SetVisibility` (`self.ToxicMesh`) true false)
      (bind (_direction _objectposition) (`Timeline|Timeline_0`)
        (:`Update`
          (`SceneComponent.K2_SetRelativeLocation` (`self.ToxicMesh`) (`KismetMathLibrary.MakeVector` 0.0 0.0 _objectposition) false false))
        (:`Finished`
          (`ActorComponent.K2_DestroyComponent` (`self.ToxicMesh`))))
      (elif (`KismetMathLibrary.Conv_IntToBool` (`KismetMathLibrary.And_IntInt` (`self.AbilitiesToUnlock`) (`|BitmaskLiteral` 2)))
        ;[1 1 1] Jetpack
        (`SceneComponent.SetVisibility` (`self.JetpackMesh`) true false)
        (`SceneComponent.SetVisibility` (`self.Jetpack2`) true false)
        (bind (_direction_2 _objectposition_2) (`Timeline|Timeline_1`)
          (:`Update`
            (`SceneComponent.K2_SetRelativeLocation` (`self.JetpackMesh`) (`KismetMathLibrary.MakeVector` -0.03804 -14.128429 _objectposition_2) false false))
          (:`Finished`
            (`ActorComponent.K2_DestroyComponent` (`self.JetpackMesh`))
            (`ActorComponent.K2_DestroyComponent` (`self.Jetpack2`))))
        (elif (`KismetMathLibrary.Conv_IntToBool` (`KismetMathLibrary.And_IntInt` (`self.AbilitiesToUnlock`) (`|BitmaskLiteral` 4)))
          ;[1 1 1] Soda
          (`SceneComponent.SetVisibility` (`self.SodaMesh`) true false)
          (bind (_direction_3 _objectposition_3) (`Timeline|Soda`)
            (:`Update`
              (`SceneComponent.K2_SetRelativeLocation` (`self.SodaMesh`) (`KismetMathLibrary.MakeVector` 0.0 0.0 _objectposition_3) false false))
            (:`Finished`
              (`ActorComponent.K2_DestroyComponent` (`self.SodaMesh`)))))))))

(fn `UserConstructionScript`)