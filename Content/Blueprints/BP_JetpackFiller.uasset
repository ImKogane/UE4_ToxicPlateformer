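; BP_JetpackFiller is a pickup that refills a player's jetpack when they touch it.
; Overlapping its box casts the other actor to HazardPlayer and calls RefillJetpack with a configurable amount in seconds.
; Only a successful refill triggers the respawn, which hides the pickup and disables its collision for a configurable delay before restoring both.
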(event `self.Box.OnComponentBeginOverlap`
  (params (OverlappedComponent :type "PrimitiveComponent Object Reference") (OtherActor :type "Actor Object Reference") (OtherComp :type "PrimitiveComponent Object Reference") (OtherBodyIndex :type Integer) (bFromSweep :type Boolean) (SweepResult :type "HitResult Structure (by ref)"))
  (bind _ashazard_player (cast `/Game/ThirdPersonBP/Blueprints/HazardPlayer` OtherActor))
  (bind _changed (`/Game/ThirdPersonBP/Blueprints/HazardPlayer.RefillJetpack` _ashazard_player (`self.AmountInSeconds`)))
  (if _changed
    (`self.StartRespawn`)))

(event `StartRespawn`
  (`self.SetActorHiddenInGame` true)
  (`self.SetActorEnableCollision` false)
  (`KismetSystemLibrary.Delay` (`self.RespawnDelay`))
  (`self.SetActorHiddenInGame` false)
  (`self.SetActorEnableCollision` true))

(fn `UserConstructionScript`)